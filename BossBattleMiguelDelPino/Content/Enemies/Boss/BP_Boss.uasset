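; Boss enemy that casts fire, ice and electric spells, teleports, summons minions and wins the game for the player on death.
; Cast and start functions only set a Style state, which CreateSpell later resolves into a projectile, area, teleport or summon (Beam).
; A randomly offset indicator near the player places area spells and the electric projectile.
; SwitchElement cycles the element, and Enrage doubles the boss's scale with attached particles.
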(event `self.ReceiveBeginPlay`
  (`parent.ReceiveBeginPlay`)
  (bind _outactors (`GameplayStatics.GetAllActorsOfClass` "/Game/Player/BP_Player.BP_Player_C"))
  (set `self.PlayerActor` (`|GetArrayItem` _outactors))
  (set `self.Style` "NewEnumerator3"))

(event `/Game/ClasesPadre/Vida.Morir`
  (`self.K2_DestroyActor`)
  (bind _asmy_game_mode (cast `/Game/MyGameMode` (`GameplayStatics.GetGameMode`)))
  (`/Game/MyGameMode.Win` _asmy_game_mode))

(fn `CastAOESpell`
  (set `self.Style` "NewEnumerator2"))

(fn `CastProyectileSpell`
  (set `self.Style` "NewEnumerator1"))

(fn `CreateIndicatorAroundPlayer`
  (bind _target (`self.Target`))
  (`/Engine/EditorBlueprintResources/StandardMacros.IsValid` _target
    (:`Is Valid`
      (`self.K2_DestroyActor` _target))
    (:`Is Not Valid`
      _))
  (bind _returnvalue (`|SpawnActorFromClass` "/Game/Enemies/Boss/BossTargetting.BossTargetting_C" (`self.GetTransform`) "Undefined" "OverrideRootScale" null null))
  (bind _output_get (set `self.Target` _returnvalue))
  (bind _randomlocation (`self.GetLocationAroundActor` (`self.PlayerActor`)))
  (`self.K2_SetActorLocation` _output_get _randomlocation false false))

(fn `CreateSpell`
  (bind _target (`self.Target`))
  (bind _returnvalue (`SceneComponent.K2_GetComponentToWorld` (`self.SpellArrow`)))
  (bind _returnvalue_2 (`KismetMathLibrary.MakeTransform` (.location (`self.GetTransform` _target)) (.rotation (`self.GetTransform` _target))))
  (switch `/Game/Enums/CastingType` (`self.Style`)
    (:`NewEnumerator0`
      (`self.Summon`))
    (:`NewEnumerator1`
      (switch `/Game/Enums/SpellElement` (`self.Element`)
        (:`NewEnumerator0`
          (`|SpawnActorFromClass` "/Game/Hechizos/Proyectiles/ProyectilFuego.ProyectilFuego_C" _returnvalue "AlwaysSpawn" "OverrideRootScale" null self))
        (:`NewEnumerator1`
          (`|SpawnActorFromClass` "/Game/Hechizos/Proyectiles/ProyectilHielo.ProyectilHielo_C" _returnvalue "AlwaysSpawn" "OverrideRootScale" null self))
        (:`NewEnumerator2`
          (`|SpawnActorFromClass` "/Game/Hechizos/Proyectiles/ProyectilElectrico.ProyectilElectrico_C" _returnvalue_2 "AlwaysSpawn" "OverrideRootScale" null self))))
    (:`NewEnumerator2`
      (`/Engine/EditorBlueprintResources/StandardMacros.IsValid` _target
        (:`Is Valid`
          (switch `/Game/Enums/SpellElement` (`self.Element`)
            (:`NewEnumerator0`
              (`|SpawnActorFromClass` "/Game/Hechizos/Areas/AreaFuego.AreaFuego_C" _returnvalue_2 "Undefined" "OverrideRootScale" null self))
            (:`NewEnumerator1`
              (`|SpawnActorFromClass` "/Game/Hechizos/Areas/AreaHielo.AreaHielo_C" _returnvalue_2 "Undefined" "OverrideRootScale" null self))
            (:`NewEnumerator2`
              (bind _returnvalue_3 (`|SpawnActorFromClass` "/Game/Hechizos/Areas/AreaElectrica.AreaElectrica_C" _returnvalue_2 "Undefined" "OverrideRootScale" null self))
              (`self.K2_AddActorWorldOffset` _returnvalue_3 (* (`KismetMathLibrary.Vector_Up`) 150.0) false true))))))
    (:`NewEnumerator4`
      (`self.Teleport`))))

(fn `Enrage`
  (bind _returnvalue (`|SpawnActorFromClass` "/Game/Enemies/Boss/ParticulasEnrage.ParticulasEnrage_C" (`SceneComponent.K2_GetComponentToWorld` (`self.EnrageArrow`)) "Undefined" "OverrideRootScale" null null))
  (`self.SetActorScale3D` (2.0 2.0 2.0))
  (`self.K2_AttachToActor` _returnvalue self "None" "KeepWorld" "KeepWorld" "KeepWorld" true))

(fn `GetLocationAroundActor`
  (params (Actor :type "Actor Object Reference"))
  (returns (RandomLocation :type "Vector Structure"))
  (bind _returnvalue (`self.K2_GetActorLocation` Actor))
  (return (`KismetMathLibrary.MakeVector` (.x (+ _returnvalue (`KismetMathLibrary.MakeVector` (`KismetMathLibrary.RandomFloatInRange` -250.0 250.0) (`KismetMathLibrary.RandomFloatInRange` -250.0 250.0)))) (.y (+ _returnvalue (`KismetMathLibrary.MakeVector` (`KismetMathLibrary.RandomFloatInRange` -250.0 250.0) (`KismetMathLibrary.RandomFloatInRange` -250.0 250.0)))) (.z _returnvalue))))

(fn `StartSummon`
  (params (Number :type Integer))
  (set `self.NumberToSummon` Number)
  (set `self.Style` "NewEnumerator0"))

(fn `StartTeleport`
  (params (Location :type "Vector Structure"))
  (set `self.TeleportLocation` Location)
  (set `self.Style` "NewEnumerator4"))

(fn `Summon`
  (for _ (range 1 (+ (`self.NumberToSummon`) 1))
    (bind _randomlocation (`self.GetLocationAroundActor` self))
    (`|SpawnActorFromClass` "/Game/Enemies/Minions/BP_Minion.BP_Minion_C" (`KismetMathLibrary.MakeTransform` _randomlocation (.rotation (`self.GetTransform`))) "AdjustIfPossibleButAlwaysSpawn" "OverrideRootScale" null 100.0 null)))

(fn `SwitchElement`
  ;[1 1 1] El boss va rotando entre elementos de forma cíclica
  (switch `/Game/Enums/SpellElement` (`self.Element`)
    (:`NewEnumerator0`
      (set `self.Element` "NewEnumerator1"))
    (:`NewEnumerator1`
      (set `self.Element` "NewEnumerator2"))
    (:`NewEnumerator2`
      (set `self.Element` "NewEnumerator0"))))

(fn `Teleport`
  (`self.K2_TeleportTo` (`self.TeleportLocation`))
  (`self.K2_SetActorRotation` (`KismetMathLibrary.FindLookAtRotation` (`self.K2_GetActorLocation`) (`self.K2_GetActorLocation` (`self.PlayerActor`)))))

(fn `UserConstructionScript`)