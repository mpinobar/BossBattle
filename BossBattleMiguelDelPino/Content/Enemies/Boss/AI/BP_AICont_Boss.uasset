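; BP_AICont_Boss is the AI controller for the boss enemy.
; On BeginPlay it loads the BB_AI_Boss blackboard and runs the BT_AI_Boss behavior tree.
; It seeds the blackboard with the first BP_Player found, an Idle style, the current phase, and the controlled BP_Boss's current shield value.
; These values are written only at startup; Tick is unused.
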(event `self.ReceiveBeginPlay`
  (bind _blackboardcomponent (`self.UseBlackboard` "/Game/Enemies/Boss/AI/BB_AI_Boss.BB_AI_Boss"))
  (`self.RunBehaviorTree` "/Game/Enemies/Boss/AI/BT_AI_Boss.BT_AI_Boss")
  (bind _outactors (`GameplayStatics.GetAllActorsOfClass` "/Game/Player/BP_Player.BP_Player_C"))
  (`BlackboardComponent.SetValueAsObject` _blackboardcomponent (`self.Player`) (`|GetArrayItem` _outactors))
  (`BlackboardComponent.SetValueAsEnum` _blackboardcomponent (`self.Style`) (`self.Idle`))
  (`BlackboardComponent.SetValueAsEnum` _blackboardcomponent (`self.FaseVar`) (`self.Fase`))
  (bind _asbp_boss (cast `/Game/Enemies/Boss/BP_Boss` (`self.K2_GetPawn`)))
  (`BlackboardComponent.SetValueAsFloat` _blackboardcomponent (`self.EscudoVar`) (`/Game/ClasesPadre/Vida.EscudoActual` _asbp_boss)))

(fn `UserConstructionScript`)