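; Minion enemy that detects the player, attacks and shows a health bar turned toward the camera.
; AI perception stores or clears the player reference and notifies Minion_AiController on detection.
; It extends parent damage and death logic, refreshing the MinionWidget after each hit and destroying itself shortly after dying.
; Attack spawns a damage-carrying attack actor at the AttackArrow transform.
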(event `self.Morir`
  (`parent.Morir`)
  (`KismetSystemLibrary.Delay` 5.0)
  (`self.K2_DestroyActor`))

(event `self.ReceiveBeginPlay`
  (`parent.ReceiveBeginPlay`)
  (set `self.MinionState` "NewEnumerator0")
  (bind _outactors (`GameplayStatics.GetAllActorsOfClass` "/Game/Player/BP_Player.BP_Player_C"))
  (set `self.Player` (`|GetArrayItem` _outactors))
  (bind _asminion_widget (cast `/Game/UI/MinionWidget` (`WidgetComponent.GetUserWidgetObject` (`self.MinionWidgetComponent`))))
  (`/Game/UI/MinionWidget.UpdateVars` _asminion_widget (`self.VidaActual`) (`self.VidaMaxima`)))

(event `self.AIPerception.OnTargetPerceptionUpdated`
  (params (Actor :type "Actor Object Reference") (Stimulus :type "AIStimulus Structure"))
  ;[1 1 1] Que el minion avise al controlador de que ha visto al jugador
  (bind _asbp_player (cast `/Game/Player/BP_Player` Actor))
  (if (`.bSuccessfullySensed` (break `AIStimulus` Stimulus))
    (set `self.Player` _asbp_player)
    (bind _asminion_ai_controller (cast `/Game/Enemies/Minions/AI/Minion_AiController` (`AIBlueprintHelperLibrary.GetAIController` self)))
    (`/Game/Enemies/Minions/AI/Minion_AiController.OnPlayerDetected` _asminion_ai_controller)
    (else
      (set `self.Player` null))))

(event `self.ReceiveTick`
  (params (DeltaSeconds :type "Float (single-precision)"))
  ;[1 1 1] Actualizar la rotación de la barra de vida
  (`SceneComponent.K2_SetWorldRotation` (`self.MinionWidgetComponent`) (`KismetMathLibrary.FindLookAtRotation` (`SceneComponent.K2_GetComponentLocation` (`self.MinionWidgetComponent`)) (`PlayerCameraManager.GetCameraLocation` (`GameplayStatics.GetPlayerCameraManager` 0))) false false))

(event `self.RestarVida`
  (params (`Daño` :type "Float (single-precision)") (`TipoDaño` :type "/Game/Enums/SpellElement Enum" :default "NewEnumerator0"))
  ;[1 1 1] Actualizar la barra de vida
  (`parent.RestarVida` `Daño` `TipoDaño`)
  (bind _asminion_widget (cast `/Game/UI/MinionWidget` (`WidgetComponent.GetUserWidgetObject` (`self.MinionWidgetComponent`))))
  (`/Game/UI/MinionWidget.UpdateVars` _asminion_widget (`self.VidaActual`) (`self.VidaMaxima`)))

(fn `Attack`
  (`|SpawnActorFromClass` "/Game/Enemies/Minions/Attack.Attack_C" (`SceneComponent.K2_GetComponentToWorld` (`self.AttackArrow`)) "Undefined" "OverrideRootScale" null (`self.DañoAtaque`) null))

(fn `UserConstructionScript`)