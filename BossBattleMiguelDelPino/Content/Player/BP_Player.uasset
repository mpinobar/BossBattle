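; Player spellcaster character with movement, four elements (fire, ice, electric, healing), projectile, beam and area spells, and teleport.
; A timer-driven camera trace places the target marker for aimed actions.
; Releasing those inputs sets CastingStyle and blocks input, leaving the spawn and teleport functions to external callers, while beams spawn after montages and drain mana on a timer.
; Costs come from MyGameMode, Godmode zeroes them, and mana regenerates without an active beam.
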(event `RecuperarMagia`
  (bind _magiamaxima (`self.MagiaMaxima`))
  ;[1 1 1] Recuperacion de magia con el tiempo
  (`/Engine/EditorBlueprintResources/StandardMacros.IsValid` (`self.CurrentBeam`)
    (:`Is Not Valid`
      (bind _output_get (set `self.Magia` (+ (`self.Magia`) (* (`self.RecuperacionDeMagiaPorSegundo`) (`self.FrecuenciaTickMagia`)))))
      (if (> _output_get _magiamaxima)
        (set `self.Magia` _magiamaxima)))))

(event `self.ReceiveBeginPlay`
  ;[1 1 1] Setup inicial
  (`parent.ReceiveBeginPlay`)
  (bind _returnvalue (`|CreateWidget` "/Game/UI/PlayerWidget.PlayerWidget_C" (`GameplayStatics.GetPlayerController` 0)))
  (`UserWidget.AddToViewport` _returnvalue 1)
  (bind _returnvalue_2 (`|SpawnActorFromClass` "/Game/Player/PlayerTarget.PlayerTarget_C" (`self.GetTransform`) "AlwaysSpawn" "OverrideRootScale" null self))
  (bind _output_get (set `self.Target` _returnvalue_2))
  (`SceneComponent.SetVisibility` (`Actor.RootComponent` _output_get) false true)
  (set `self.CastingStyle` "NewEnumerator3")
  (set `self.Magia` (`self.MagiaMaxima`))
  (`KismetSystemLibrary.K2_SetTimer` null "RecuperarMagia" (`self.FrecuenciaTickMagia`) true))

(event `InputAxis|Forward`
  (params (AxisValue :type "Float (single-precision)"))
  ;[1 1 1] Inputs de movimiento
  (if (not (`self.BlockedInput`))
    (`self.AddMovementInput` (`KismetMathLibrary.GetForwardVector` (`self.GetControlRotation`)) AxisValue)
    (`self.MakeNoise` 1.0 null (`self.K2_GetActorLocation`) :!label _label)))

(event `InputAxis|SideMovement`
  (params (AxisValue :type "Float (single-precision)"))
  ;[1 1 1] Inputs de movimiento
  (if (not (`self.BlockedInput`))
    (`self.AddMovementInput` (`KismetMathLibrary.GetRightVector` (`self.GetControlRotation`)) AxisValue)
    (goto _label)))

(event `InputAxis|HorizontalMouse`
  (params (AxisValue :type "Float (single-precision)"))
  ;[1 1 1] Inputs de movimiento
  (if (not (`self.BlockedInput`))
    (`PlayerController.AddYawInput` (`GameplayStatics.GetPlayerController` 0) AxisValue)))

(event `InputAxis|VerticalMouse`
  (params (AxisValue :type "Float (single-precision)"))
  ;[1 1 1] Inputs de movimiento
  (`PlayerController.AddPitchInput` (`GameplayStatics.GetPlayerController` 0) (* AxisValue -1.0)))

(event `StartTargetting`
  ;[1 1 1] Sistema de apuntado con partículas
  ;;[1 1 1] Es igual que event tick
  (bind _returnvalue (`KismetSystemLibrary.K2_SetTimerDelegate` (delegate `Targetting`) 0.01 true)))

(event `Targetting`
  (bind _camera (`self.Camera`))
  (bind _target (`self.Target`))
  (bind _returnvalue (`SceneComponent.K2_GetComponentLocation` _camera))
  ;[1 1 1] Sistema de apuntado con partículas
  (bind _outactors (`GameplayStatics.GetAllActorsOfClass` "BP_Player_C"))
  (bind (_outhit _returnvalue_2) (`KismetSystemLibrary.LineTraceSingle` (+ _returnvalue (0.0 0.0 100.0)) (+ _returnvalue (* (`SceneComponent.GetForwardVector` _camera) (`self.RangoHechizos`))) "TraceTypeQuery2" false _outactors))
  (if _returnvalue_2
    (`self.K2_SetActorLocation` _target (+ (`.Location` (`GameplayStatics.BreakHitResult` _outhit)) (0.0 0.0 10.0)) false false)
    (`SceneComponent.SetVisibility` (`Actor.RootComponent` _target) true true)))

(event `EndTargetting`
  ;[1 1 1] Sistema de apuntado con partículas
  (`KismetSystemLibrary.K2_ClearAndInvalidateTimerHandle` (stale `StartTargetting` _returnvalue)))

(event `InputAction|Proyectile`
  (params (Key :type "Key Structure"))
  ;[1 1 1] Inputs de hechizos
  (:`Pressed`
    (`self.StartTargetting`)
    (`self.ComienzoDeCasteo`))
  (:`Released`
    (if (`|EnumEquality` (`self.CastingStyle`) "NewEnumerator3")
      (bind _coste (`self.GetSpellCost` "NewEnumerator1"))
      (if (<= _coste (`self.Magia`))
        (set `self.BlockedInput` true)
        (`self.EndTargetting`)
        (set `self.CastingStyle` "NewEnumerator1")))))

(event `InputAction|BeamEffect`
  (params (Key :type "Key Structure"))
  (bind _currentbeam (`self.CurrentBeam`))
  (bind _blockedinput (`self.BlockedInput`))
  (bind _mesh (`self.Mesh`))
  ;[1 1 1] Inputs de hechizos
  (:`Pressed`
    (if (not _blockedinput)
      (bind _coste (`self.GetSpellCost` "NewEnumerator0"))
      (if (<= _coste (`self.Magia`))
        (`self.ComienzoDeCasteo`)
        (set `self.CastingStyle` "NewEnumerator0")
        (`|PlayMontage` _mesh "/Game/Player/Animations/StartCasting.StartCasting"
          (:`then`
            (`|PlayMontage` (`self.Mesh`) "/Game/Player/Animations/IdleCastingMontage.IdleCastingMontage"
              (:`then`
                (`/Engine/EditorBlueprintResources/StandardMacros.DoOnce` false :!label _label_2
                  (:`Completed`
                    (`self.SpawnBeam`)
                    (bind _returnvalue (`KismetSystemLibrary.K2_SetTimerDelegate` (delegate `BeamCost`) 0.1 true)))))))))))
  (:`Released`
    (if (not (or _blockedinput (`|EnumEquality` (`self.CastingStyle`) "NewEnumerator3")))
      (`/Engine/EditorBlueprintResources/StandardMacros.IsValid` _currentbeam :!label _label_3
        (:`Is Valid`
          (`self.K2_DestroyActor` _currentbeam))
        (:`Is Not Valid`
          _))
      (set `self.CastingStyle` "NewEnumerator3")
      (`self.StopAnimMontage` "/Game/Player/Animations/IdleCastingMontage.IdleCastingMontage")
      (`|PlayMontage` _mesh "/Game/Player/Animations/EndCastingBeam.EndCastingBeam"
        (:`then`
          (`|ExecutionSequence`
            (:`then_0`
              (goto _label_2 :!via `Reset`))
            (:`then_1`
              (`KismetSystemLibrary.K2_ClearAndInvalidateTimerHandle` _returnvalue :!label _label_4))))))))

(event `BeamCost`
  ;[1 1 1] Inputs de hechizos
  (bind _coste (`self.GetSpellCost` "NewEnumerator0"))
  (bind _output_get (set `self.Magia` (- (`self.Magia`) _coste)))
  (if (<= _output_get 0.0)
    (`|ExecutionSequence`
      (:`then_0`
        (goto _label_4))
      (:`then_1`
        (goto _label_3)))))

(event `InputAction|AreaSpell`
  (params (Key :type "Key Structure"))
  ;[1 1 1] Inputs de hechizos
  (:`Pressed`
    (`self.StartTargetting`)
    (`self.ComienzoDeCasteo`))
  (:`Released`
    (if (`|EnumEquality` (`self.CastingStyle`) "NewEnumerator3")
      (bind _coste (`self.GetSpellCost` "NewEnumerator2"))
      (if (<= _coste (`self.Magia`))
        (set `self.BlockedInput` true)
        (`self.EndTargetting`)
        (set `self.CastingStyle` "NewEnumerator2")))))

(event `InputAction|FireType`
  (params (Key :type "Key Structure"))
  ;[1 1 1] Cambiar el elemento del hechizo
  (:`Pressed`
    (set `self.TypeToCast` "NewEnumerator0")
    (`self.ComienzoDeCasteo`)))

(event `InputAction|IceType`
  (params (Key :type "Key Structure"))
  ;[1 1 1] Cambiar el elemento del hechizo
  (:`Pressed`
    (set `self.TypeToCast` "NewEnumerator1")
    (`self.ComienzoDeCasteo`)))

(event `InputAction|ElectricType`
  (params (Key :type "Key Structure"))
  ;[1 1 1] Cambiar el elemento del hechizo
  (:`Pressed`
    (set `self.TypeToCast` "NewEnumerator2")
    (`self.ComienzoDeCasteo`)))

(event `InputAction|Defense`
  (params (Key :type "Key Structure"))
  ;[1 1 1] Cambiar el elemento del hechizo
  (:`Pressed`
    (set `self.TypeToCast` "NewEnumerator3")
    (`self.ComienzoDeCasteo`)))

(event `InputAction|Invulnerable`
  (params (Key :type "Key Structure"))
  ;[1 1 1] OtrosInputs
  (:`Pressed`
    (set `self.Godmode` (not (`self.Godmode`)))))

(event `InputAction|Teleport`
  (params (Key :type "Key Structure"))
  ;[1 1 1] OtrosInputs
  (:`Pressed`
    (`self.StartTargetting`))
  (:`Released`
    (if (`|EnumEquality` (`self.CastingStyle`) "NewEnumerator3")
      (set `self.BlockedInput` true)
      (`self.EndTargetting`)
      (set `self.CastingStyle` "NewEnumerator4"))))

(event `InputAction|Run`
  (params (Key :type "Key Structure"))
  ;[1 1 1] OtrosInputs
)

(event `self.Morir`
  (`parent.Morir`)
  (set `self.Dead` true)
  (set `self.BlockedInput` true)
  (bind _asmy_game_mode (cast `/Game/MyGameMode` (`GameplayStatics.GetGameMode`)))
  (`/Game/MyGameMode.RestartLevel` _asmy_game_mode))

(fn `ComienzoDeCasteo`
  (bind _returnvalue (`SceneComponent.GetSocketTransform` (`self.Mesh`) "SpellSocket" "RTS_World"))
  (`/Engine/EditorBlueprintResources/StandardMacros.IsValid` (`self.ParticulasCast`)
    (:`Is Valid`
      (`self.K2_DestroyActor` (`self.ParticulasCast`)))
    (:`Is Not Valid`
      _))
  (switch `/Game/Enums/SpellElement` (`self.TypeToCast`)
    (:`NewEnumerator0`
      (bind _returnvalue_2 (`|SpawnActorFromClass` "/Game/Hechizos/Casteos/CastFuego.CastFuego_C" _returnvalue "AlwaysSpawn" "OverrideRootScale" null null))
      (set `self.ParticulasCast` _returnvalue_2))
    (:`NewEnumerator1`
      (bind _returnvalue_3 (`|SpawnActorFromClass` "/Game/Hechizos/Casteos/CastHielo.CastHielo_C" _returnvalue "AlwaysSpawn" "OverrideRootScale" null null))
      (set `self.ParticulasCast` _returnvalue_3))
    (:`NewEnumerator2`
      (bind _returnvalue_4 (`|SpawnActorFromClass` "/Game/Hechizos/Casteos/CastElectrico.CastElectrico_C" _returnvalue "AlwaysSpawn" "OverrideRootScale" null null))
      (set `self.ParticulasCast` _returnvalue_4))
    (:`NewEnumerator3`
      (bind _returnvalue_5 (`|SpawnActorFromClass` "/Game/Hechizos/Casteos/CastCuracion.CastCuracion_C" _returnvalue "AlwaysSpawn" "OverrideRootScale" null null))
      (set `self.ParticulasCast` _returnvalue_5)))
  (`SceneComponent.K2_AttachToComponent` (`Actor.RootComponent` (`self.ParticulasCast`)) (`self.Mesh`) "SpellSocket" "SnapToTarget" "SnapToTarget" "SnapToTarget" true))

(fn `GetSpellCost`
  (params (Style :type "/Game/Enums/CastingType Enum" :default "NewEnumerator0"))
  (returns (Coste :type "Float (double-precision)"))
  (locals (Gm :type "/Game/MyGameMode Object Reference"))
  (bind _gm (`local.Gm`))
  (bind _gm_2 (`local.Gm`))
  (bind _gm_3 (`local.Gm`))
  (if (`self.Godmode`)
    (return 0.0)
    (else
      (bind _asmy_game_mode (cast `/Game/MyGameMode` (`GameplayStatics.GetGameMode`)))
      (set `local.Gm` _asmy_game_mode)
      (switch `/Game/Enums/CastingType` Style
        (:`NewEnumerator0`
          (switch `/Game/Enums/SpellElement` (`self.TypeToCast`)
            (:`NewEnumerator0`
              (return (`/Game/MyGameMode.CosteBeamFuego` _gm_3)))
            (:`NewEnumerator1`
              (return (`/Game/MyGameMode.CosteBeamHielo` _gm_3)))
            (:`NewEnumerator2`
              (return (`/Game/MyGameMode.CosteBeamElectrico` _gm_3)))
            (:`NewEnumerator3`
              (return (`/Game/MyGameMode.CosteCuracionMantenida` _gm_3)))))
        (:`NewEnumerator1`
          (switch `/Game/Enums/SpellElement` (`self.TypeToCast`)
            (:`NewEnumerator0`
              (return (`/Game/MyGameMode.CosteProyectilFuego` _gm)))
            (:`NewEnumerator1`
              (return (`/Game/MyGameMode.CosteProyectilHielo` _gm)))
            (:`NewEnumerator2`
              (return (`/Game/MyGameMode.CosteProyectilElectrico` _gm)))
            (:`NewEnumerator3`
              (return (`/Game/MyGameMode.CosteBurstCuracion` _gm)))))
        (:`NewEnumerator2`
          (switch `/Game/Enums/SpellElement` (`self.TypeToCast`)
            (:`NewEnumerator0`
              (return (`/Game/MyGameMode.CosteAreaFuego` _gm_2)))
            (:`NewEnumerator1`
              (return (`/Game/MyGameMode.CosteAreaHielo` _gm_2)))
            (:`NewEnumerator2`
              (return (`/Game/MyGameMode.CosteAreaElectrico` _gm_2)))
            (:`NewEnumerator3`
              (return (`/Game/MyGameMode.CosteAreaCuracion` _gm_2)))))))))

(fn `SpawnAOE`
  (bind _returnvalue (`self.GetTransform` (`self.Target`)))
  (bind _returnvalue_2 (+ (`SceneComponent.K2_GetComponentLocation` (`/Game/Player/PlayerTarget.DefaultSceneRoot` (`self.Target`))) (0.0 0.0 100.0)))
  (switch `/Game/Enums/SpellElement` (`self.TypeToCast`)
    (:`NewEnumerator0`
      (`|SpawnActorFromClass` "/Game/Hechizos/Areas/AreaFuego.AreaFuego_C" _returnvalue "AlwaysSpawn" "OverrideRootScale" null null))
    (:`NewEnumerator1`
      (`|SpawnActorFromClass` "/Game/Hechizos/Areas/AreaHielo.AreaHielo_C" _returnvalue "AlwaysSpawn" "OverrideRootScale" null null))
    (:`NewEnumerator2`
      (bind _returnvalue_3 (`|SpawnActorFromClass` "/Game/Hechizos/Areas/AreaElectrica.AreaElectrica_C" _returnvalue "AlwaysSpawn" "OverrideRootScale" null null))
      (`self.K2_SetActorRotation` _returnvalue_3 (`self.K2_GetActorRotation` (`GameplayStatics.GetPlayerPawn` 0)) false)
      (`self.K2_SetActorLocation` _returnvalue_3 _returnvalue_2 false false))
    (:`NewEnumerator3`
      (bind _returnvalue_4 (`|SpawnActorFromClass` "/Game/Hechizos/Curaciones/AreaCuracion.AreaCuracion_C" _returnvalue "AlwaysSpawn" "OverrideRootScale" null null))
      (`self.K2_SetActorLocation` _returnvalue_4 _returnvalue_2 false false)))
  (bind _coste (`self.GetSpellCost` "NewEnumerator2"))
  (set `self.Magia` (- (`self.Magia`) _coste)))

(fn `SpawnBeam`
  (bind _returnvalue (`SceneComponent.K2_GetComponentToWorld` (`self.BeamArrow`)))
  (switch `/Game/Enums/SpellElement` (`self.TypeToCast`)
    (:`NewEnumerator0`
      (bind _returnvalue_2 (`|SpawnActorFromClass` "/Game/Hechizos/Beams/BeamFuego.BeamFuego_C" _returnvalue "Undefined" "OverrideRootScale" null null))
      (set `self.CurrentBeam` _returnvalue_2))
    (:`NewEnumerator1`
      (bind _returnvalue_3 (`|SpawnActorFromClass` "/Game/Hechizos/Beams/BeamHielo.BeamHielo_C" _returnvalue "Undefined" "OverrideRootScale" null null))
      (set `self.CurrentBeam` _returnvalue_3))
    (:`NewEnumerator2`
      (bind _returnvalue_4 (`|SpawnActorFromClass` "/Game/Hechizos/Beams/BeamElectrico.BeamElectrico_C" _returnvalue "Undefined" "OverrideRootScale" null null))
      (set `self.CurrentBeam` _returnvalue_4))
    (:`NewEnumerator3`
      (bind _returnvalue_5 (`|SpawnActorFromClass` "/Game/Hechizos/Curaciones/CuracionMantenida.CuracionMantenida_C" (`self.GetTransform`) "Undefined" "OverrideRootScale" null null))
      (set `self.CurrentBeam` _returnvalue_5)))
  (`SceneComponent.K2_AttachToComponent` (`Actor.RootComponent` (`self.CurrentBeam`)) (`self.Mesh`) "None" "KeepWorld" "KeepWorld" "KeepWorld" true))

(fn `SpawnProjectile`
  (bind _returnvalue (`self.GetTransform`))
  (switch `/Game/Enums/SpellElement` (`self.TypeToCast`)
    (:`NewEnumerator0`
      (`|SpawnActorFromClass` "/Game/Hechizos/Proyectiles/ProyectilFuego.ProyectilFuego_C" _returnvalue "AlwaysSpawn" "OverrideRootScale" null null))
    (:`NewEnumerator1`
      (`|SpawnActorFromClass` "/Game/Hechizos/Proyectiles/ProyectilHielo.ProyectilHielo_C" _returnvalue "AlwaysSpawn" "OverrideRootScale" null null))
    (:`NewEnumerator2`
      (bind _returnvalue_2 (`|SpawnActorFromClass` "/Game/Hechizos/Proyectiles/ProyectilElectrico.ProyectilElectrico_C" _returnvalue "AlwaysSpawn" "OverrideRootScale" null null))
      (`self.K2_SetActorLocation` _returnvalue_2 (`SceneComponent.K2_GetComponentLocation` (`/Game/Player/PlayerTarget.DefaultSceneRoot` (`self.Target`))) false false))
    (:`NewEnumerator3`
      (bind _returnvalue_3 (`|SpawnActorFromClass` "/Game/Hechizos/Curaciones/BurstCuracion.BurstCuracion_C" _returnvalue "AlwaysSpawn" "OverrideRootScale" null null))
      (`SceneComponent.K2_AttachToComponent` (`Actor.RootComponent` _returnvalue_3) (`self.Mesh`) "None" "KeepWorld" "KeepWorld" "KeepWorld" true)))
  (bind _coste (`self.GetSpellCost` "NewEnumerator1"))
  (set `self.Magia` (- (`self.Magia`) _coste)))

(fn `Teleport`
  (`self.K2_TeleportTo` (`self.K2_GetActorLocation` (`self.Target`))))

(fn `UserConstructionScript`)